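; Multiplayer game instance that handles connection failures and leaving online sessions.
; Network and travel error events print the failure type for debugging, then share one path that destroys the first player controller's session.
; LeaveSession opens the VR template map by name, then destroys the session.
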(event Custom|LeaveSession
  ;[1 1 1] Leave Session
  (Game|OpenLevel(byName) "VRTemplateMap")
  (|DestroySession (Game|GetPlayerController 0)))

(event EventHandleNetworkError
  (params (FailureType :type ENetworkFailure%20Enum :default "NetDriverAlreadyExists") (bIsServer :type Boolean))
  ;[1 1 1] Debug
  (Development|PrintString (Utilities|String|EnumtoString FailureType))
  (|DestroySession (Game|GetPlayerController 0)))

(event EventHandleTravelError
  (params (FailureType :type ETravelFailure%20Enum :default "NoLevel"))
  ;[1 1 1] Debug
  (Development|PrintString (Utilities|String|EnumtoString FailureType))
  (|DestroySession (Game|GetPlayerController 0)))