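; BP_GM_Main is a multiplayer game mode that tracks connected players and supports kicking them.
; It adds and removes BP_PC_main controllers in a JoinedPlayers array on login and logout, then after a short delay has BP_GS_Main update the player list.
; KickPlayer uses the given ID as an index into that array and calls OwningClientKickPlayer on that controller.
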(event Custom|UpdatePlayerList
  (Utilities|FlowControl|Delay 0.5)
  (bind _asbp_gs_main (Utilities|Casting|CastToBP_GS_Main (Game|GetGameState)))
  (Default|UpdatePlayerList _asbp_gs_main))

(event EventBeginPlay)

(event EventTick
  (params (DeltaSeconds :type Float%20%28single-precision%29)))

(event EventPostLogin
  (params (NewPlayer :type Player%20Controller%20Object%20Reference))
  (bind _asbp_pc_main (Utilities|Casting|CastToBP_PC_main NewPlayer))
  (Utilities|Array|Add (Variables|Default|GetJoinedPlayers) _asbp_pc_main)
  (CallFunction|UpdatePlayerList))

(event EventOnLogout
  (params (ExitingController :type Controller%20Object%20Reference))
  (bind _asbp_pc_main (Utilities|Casting|CastToBP_PC_main ExitingController))
  (Utilities|Array|RemoveItem (Variables|Default|GetJoinedPlayers) _asbp_pc_main)
  (CallFunction|UpdatePlayerList))

(fn ConstructionScript)

(fn KickPlayer
  (params (PlayerId :type Integer))
  (Default|OwningClientKickPlayer (Utilities|Array|Get(acopy) (Variables|Default|GetJoinedPlayers) PlayerId)))