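; Multiplayer game state that keeps open player-list menus in sync with the connected players.
; UpdatePlayerList copies PlayerArray into the replicated AllPLayerStates variable.
; Its OnRep searches all VRPawns for a valid MenuReference and calls UpdateList on that menu's WB_playerListAndLeave widget.
; An alternative refresh through a search of top-level widgets is left disconnected.
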(event Custom|UpdatePlayerList
  (Variables|Default|SetAllPLayerStates (Variables|Default|GetPlayerArray)))

(event EventBeginPlay)

(event EventTick
  (params (DeltaSeconds :type Float%20%28single-precision%29)))

(fn ConstructionScript)

(fn OnRepAllPLayerStates
  ;[1 1 1] Update Player List any time menu is open
  (bind _outactors (Actor|GetAllActorsOfClass "/Game/Multiplayer/VRTemplate/Blueprints/VRPawn.VRPawn_C"))
  (for _array_element _outactors
    (bind _menureference (Variables|/Game/Multiplayer/VRTemplate/Blueprints/VRPawn.VRPawn_C|GetMenuReference _array_element)
      (:then
        (bind _aswb_player_list_and_leave (Utilities|Casting|CastToWB_playerListAndLeave (UserInterface|GetWidget (Variables|/Game/Multiplayer/VRTemplate/Blueprints/Menu.Menu_C|GetWidget _menureference))))
        (Default|UpdateList _aswb_player_list_and_leave))
      (:else))))